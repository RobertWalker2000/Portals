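; BP_PortalPlacementChecker is a helper that tests whether a position on a surface is valid for placing a portal.
; CheckForOverlaps reads the actors overlapping its OverlapDetector component and fails if any is other than itself or the given surface.
; It has no active event logic, so the check runs only when the function is called.
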(fn `CheckForOverlaps`
  (params (Surface :type "Actor Object Reference"))
  (returns (IsValid :type Boolean))
  (for _array_element (`PrimitiveComponent.GetOverlappingActors` (`self.OverlapDetector`) null)
    (if (not (or (== Surface _array_element) (== _array_element self)))
      (return false)))
  (return true))

(fn `UserConstructionScript`
  (`parent.UserConstructionScript`))