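; Portal gun that fires portals onto surfaces the player aims at, using its owner's camera.
; On FirePortal, a long visibility line trace from the camera finds the hit point and surface normal.
; A temporary BP_PortalPlacementChecker spawns there, facing along the normal, letting spawn collision handling nudge or reject the placement.
; If it spawns, its transform is kept, the checker is destroyed and BP_PortalBase spawns at that transform.
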(event `self.ReceiveBeginPlay`
  (bind _returnvalue (`Actor.GetComponentByClass` (`self.GetOwner` self) "/Script/Engine.CameraComponent"))
  (`/Engine/EditorBlueprintResources/StandardMacros.IsValid` _returnvalue
    (:`Is Valid`
      (set `self.Camera` _returnvalue))))

(event `InputAction|FirePortal`
  (params (Key :type "Key Structure"))
  (:`Pressed`
    (bind _hit (`self.Trace Shot`))
    (if (`GameplayStatics.BreakHitResult` _hit)
      (bind (_ispositionvalid _newtransform) (`self.CheckPosition` (`.Location` (`GameplayStatics.BreakHitResult` _hit)) (`.Normal` (`GameplayStatics.BreakHitResult` _hit)) (`.HitActor` (`GameplayStatics.BreakHitResult` _hit))))
      (if _ispositionvalid
        (`self.Spawn Portal` _newtransform)))))

(fn `CheckPosition`
  (params (SpawnPoint :type "Vector Structure") (`Portal Forward` :type "Vector Structure") (Surface :type "Actor Object Reference"))
  (returns (IsPositionValid :type Boolean) (NewTransform :type "Transform Structure"))
  (locals (PortalChecker :type "/Game/Portals/Blueprints/Portals/BP_PortalPlacementChecker Object Reference") (PortalTransform :type "Transform Structure"))
  (bind _returnvalue (`|SpawnActorFromClass` "/Game/Portals/Blueprints/Portals/BP_PortalPlacementChecker.BP_PortalPlacementChecker_C" (`KismetMathLibrary.MakeTransform` SpawnPoint (`KismetMathLibrary.Conv_VectorToRotator` `Portal Forward`)) "AdjustIfPossibleButDontSpawnIfColliding" "OverrideRootScale" null null))
  (`/Engine/EditorBlueprintResources/StandardMacros.IsValid` _returnvalue
    (:`Is Valid`
      (bind _output_get (set `local.PortalChecker` _returnvalue))
      (bind _output_get_2 (set `local.PortalTransform` (`Actor.GetTransform` _output_get)))
      (`Actor.K2_DestroyActor` (`local.PortalChecker`))
      (return true _output_get_2))))

(fn `Spawn Portal`
  (params (PortalTransform :type "Transform Structure"))
  (`|SpawnActorFromClass` "/Game/Portals/Blueprints/Portals/BP_PortalBase.BP_PortalBase_C" PortalTransform "Undefined" "OverrideRootScale" null null))

(fn `Trace Shot`
  (returns (Hit :type "HitResult Structure"))
  (bind _camera (`self.Camera`))
  (bind _returnvalue (`SceneComponent.K2_GetComponentLocation` _camera))
  (bind _outhit (`KismetSystemLibrary.LineTraceSingle` :`Start` _returnvalue :`End` (+ _returnvalue (* (`SceneComponent.GetForwardVector` _camera) (`KismetMathLibrary.Conv_DoubleToVector` 50000.0))) :`TraceChannel` "TraceTypeQuery1" :`DrawDebugType` "ForDuration")) ; Check for the first collision along the generated line
  (return _outhit))